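; BP_GameMode is the game mode that opens a round of a hydra-themed party game.
; On BeginPlay it shows W_RoundCounter for two seconds under UI-only input, then restores game-only input, while background music starts without waiting.
; An unconnected graph would spawn one colored BP_HydraHead per player through SpawnHeads, which picks randomly among four TargetPoints without preventing repeats.
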(event EventBeginPlay
  (bind _returnvalue (Game|GetPlayerController 0))
  (Variables|/Script/Engine.PlayerController|SetbShowMouseCursor _returnvalue false)
  (Input|SetInputModeUIOnly _returnvalue 0 "DoNotLock")
  (Utilities|FlowControl|Sequence
    (:then_1
      (bind _returnvalue_2 (UserInterface|CreateWidget "/Game/Blueprints/Widgets/W_RoundCounter.W_RoundCounter_C"))
      (bind _output_get (Variables|Default|SetRoundCounter _returnvalue_2))
      (UserInterface|Viewport|AddtoViewport _output_get 0)
      (Utilities|FlowControl|Delay 2.0)
      (Widget|RemovefromParent _output_get)
      (Input|SetInputModeGameOnly (Game|GetPlayerController 0)))
    (:then_2
      (Audio|PlaySound2D "/Game/Audio/greek_hydra_party_background_music.greek_hydra_party_background_music" 1.0 1.0 0.0 0 0))))

(fn ConstructionScript)

(fn SpawnHeads
  (bind _outactors (Actor|GetAllActorsOfClass "/Script/Engine.TargetPoint"))
  (bind _output_get (Variables|Default|SetSpawnPoints _outactors))
  (bind _returnvalue (Game|SpawnActorfromClass "/Game/Blueprints/BP_HydraHead.BP_HydraHead_C" (Transformation|GetActorTransform (Utilities|Array|Get(acopy) _output_get (Math|Random|RandomIntegerinRange 0 3))) "Undefined" 0 0))
  (return (Variables|/Game/Blueprints/BP_HydraHead.BP_HydraHead_C|GetSkeletalMesh1 _returnvalue)))