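; Hydra head actor that multiplies when killed, in the style of the mythical Hydra.
; Any damage lowers its health; at zero or below it waits briefly, destroys itself and plays a slash particle effect at its location.
; It then calls SpawnHeads on BP_GameMode twice, leaving the creation of replacement heads to the game mode.
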(event Game|Damage|EventAnyDamage
  (params (Damage :type Float%20%28single-precision%29) (DamageType :type Damage%20Type%20Object%20Reference) (InstigatedBy :type Controller%20Object%20Reference) (DamageCauser :type Actor%20Object%20Reference))
  ;[1 0.02781 0] Take Damage
  (bind _output_get (Variables|Default|SetHealthVal (- (Variables|Default|GetHealthVal) Damage)))
  (if (<= _output_get 0.0)
    ;[0 0.2316 1] Spawn New Head + Kill older head
    (bind _asbp_game_mode (Utilities|Casting|CastToBP_GameMode (Game|GetGameMode)))
    (Utilities|FlowControl|Delay 0.1)
    (Actor|DestroyActor)
    (Effects|SpawnEmitteratLocation "/Game/Particles/P_Slash.P_Slash" (Transformation|GetActorLocation))
    (for _index (range 0 1)
      (Default|SpawnHeads _asbp_game_mode))))

(fn ConstructionScript)