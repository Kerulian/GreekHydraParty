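; BP_SwordZone is an actor that periodically damages BP_HydraHead actors inside its damage boxes.
; On BeginPlay it fills an array with four boxes, then starts an endless loop with a three-second Delay.
; Each pass picks a random box and applies one point of damage to the first overlapping hydra head.
; It does not check whether that box has any overlap.
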(event EventBeginPlay
  ;[0 0.01242 1] Damage Boxes Array Init
  (Variables|Default|SetBoxDamage (Utilities|Array|MakeArray (Variables|Default|Get1.0) (Variables|Default|Get0.0) (Variables|Default|Get0.1) (Variables|Default|Get1.1)))
  ;[1 0 0.05111] Damage done -> Recursion
  (Utilities|FlowControl|Delay 3.0 :!label _label)
  (Game|Damage|ApplyDamage (Utilities|Array|Get(acopy) (Collision|GetOverlappingActors (Utilities|Array|Get(acopy) (Variables|Default|GetBoxDamage) (Math|Random|RandomIntegerinRange 0 3)) "/Game/Blueprints/BP_HydraHead.BP_HydraHead_C" :!class /Script/Engine.PrimitiveComponent)) 1.0 0 0)
  (goto _label))

(fn ConstructionScript)